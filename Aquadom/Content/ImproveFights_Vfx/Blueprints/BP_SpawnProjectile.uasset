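; BP_SpawnProjectile is a spawner actor that repeatedly fires three projectile classes in turn from its own transform, apparently to showcase VFX.
; After a configurable start delay on BeginPlay, a switch on IncLevel picks the class and advances the counter, resetting after the third.
; The Again event re-calls itself through Delays to form an endless loop, with a longer pause after the third projectile.
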(event `Again`
  (bind _returnvalue (`self.GetTransform`))
  (switch `int` (`self.IncLevel`) :!label _label
    (:`Default`
      (`|SpawnActorFromClass` (`self.Projectile_03`) _returnvalue "Undefined" "SelectDefaultAtRuntime" null null :!label _label_2)
      (set `self.IncLevel` 0)
      (`KismetSystemLibrary.Delay` 8.5))
    (:`0`
      (`|SpawnActorFromClass` (`self.Projectile`) _returnvalue "Undefined" "SelectDefaultAtRuntime" null null)
      (set `self.IncLevel` 1))
    (:`1`
      (`|SpawnActorFromClass` (`self.Projectile_02`) _returnvalue "Undefined" "SelectDefaultAtRuntime" null null)
      (set `self.IncLevel` 2))
    (:`2`
      (goto _label_2)))
  (`KismetSystemLibrary.Delay` 1.2)
  (`self.Again`))

(event `self.ReceiveBeginPlay`
  (`KismetSystemLibrary.Delay` (`self.ExampleDelay`))
  (goto _label))

(fn `UserConstructionScript`)